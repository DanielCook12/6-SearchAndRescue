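; Hostage3 is a flipbook-animated hostage character that follows the player on the X-Z plane when in range.
; Overlapping DetectSphere steers it toward the player's capsule, while overlapping DetectSphere2 overrides this with zero movement.
; Each tick it passes itself and whether either sphere overlaps to PlayerCharacter as Hostage3 and IsHoldingHostage3.
; Location samples taken around a one-frame Delay select the directional flipbook, with idle used at zero velocity.
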(event `self.ReceiveTick`
  (params (DeltaSeconds :type "Float (single-precision)"))
  (bind _returnvalue (`self.K2_GetActorLocation`))
  (bind (_returnvalue_x _returnvalue_y _returnvalue_z) (`KismetMathLibrary.BreakVector` (`SceneComponent.K2_GetComponentLocation` (`self.CapsuleComponent`))))
  (`/Engine/EditorBlueprintResources/StandardMacros.IsValid` self
    (:`Is Valid`
      (`|ExecutionSequence`
        (:`then_0`
          (`|ExecutionSequence`
            (:`then_0`
              (set `self.oldHostageLocation` _returnvalue))
            (:`then_1`
              (`KismetSystemLibrary.Delay` DeltaSeconds)
              (set `self.currentHostageLocation` _returnvalue))))
        (:`then_1`
          (`self.hostageAnimUpdate`))
        (:`then_2`
          (if (`self.isOverlapping2`)
            (`self.AddMovementInput` (0.0 0.0 0.0))
            (elif (`self.isOverlapping`)
              (bind _asplayer_character (cast `/Game/Blueprints/PlayerCharacter` (`GameplayStatics.GetPlayerCharacter` 0)))
              (bind (_returnvalue_x_2 _returnvalue_y_2 _returnvalue_z_2) (`KismetMathLibrary.BreakVector` (`SceneComponent.K2_GetComponentLocation` (`Character.CapsuleComponent` _asplayer_character))))
              (`self.AddMovementInput` (`KismetMathLibrary.MakeVector` (- _returnvalue_x_2 _returnvalue_x) 0.0 (- _returnvalue_z_2 _returnvalue_z)))
              (else
                (`self.AddMovementInput` (0.0 0.0 0.0) 0.0)))))
        (:`then_3`
          (bind _asplayer_character_2 (cast `/Game/Blueprints/PlayerCharacter` (`GameplayStatics.GetPlayerCharacter` 0)))
          (set `/Game/Blueprints/PlayerCharacter.IsHoldingHostage3` (or (`self.isOverlapping`) (`self.isOverlapping2`)) _asplayer_character_2)
          (set `/Game/Blueprints/PlayerCharacter.Hostage3` self _asplayer_character_2))))))

(event `self.detectSphere.OnComponentBeginOverlap`
  (params (OverlappedComponent :type "PrimitiveComponent Object Reference") (OtherActor :type "Actor Object Reference") (OtherComp :type "PrimitiveComponent Object Reference") (OtherBodyIndex :type Integer) (bFromSweep :type Boolean) (SweepResult :type "HitResult Structure (by ref)"))
  (if (== OtherActor (`GameplayStatics.GetPlayerCharacter` 0))
    (set `self.isOverlapping` true)))

(event `self.detectSphere.OnComponentEndOverlap`
  (params (OverlappedComponent :type "PrimitiveComponent Object Reference") (OtherActor :type "Actor Object Reference") (OtherComp :type "PrimitiveComponent Object Reference") (OtherBodyIndex :type Integer))
  (if (== OtherActor (`GameplayStatics.GetPlayerCharacter` 0))
    (set `self.isOverlapping` false)))

(event `self.detectSphere2.OnComponentBeginOverlap`
  (params (OverlappedComponent :type "PrimitiveComponent Object Reference") (OtherActor :type "Actor Object Reference") (OtherComp :type "PrimitiveComponent Object Reference") (OtherBodyIndex :type Integer) (bFromSweep :type Boolean) (SweepResult :type "HitResult Structure (by ref)"))
  (if (== OtherActor (`GameplayStatics.GetPlayerCharacter` 0))
    (set `self.isOverlapping2` true)))

(event `self.detectSphere2.OnComponentEndOverlap`
  (params (OverlappedComponent :type "PrimitiveComponent Object Reference") (OtherActor :type "Actor Object Reference") (OtherComp :type "PrimitiveComponent Object Reference") (OtherBodyIndex :type Integer))
  (if (== OtherActor (`GameplayStatics.GetPlayerCharacter` 0))
    (set `self.isOverlapping2` false)))

(fn `hostageAnimUpdate`
  (bind (_currenthostagelocation_x _currenthostagelocation_y _currenthostagelocation_z) (`KismetMathLibrary.BreakVector` (`self.currentHostageLocation`)))
  (bind (_oldhostagelocation_x _oldhostagelocation_y _oldhostagelocation_z) (`KismetMathLibrary.BreakVector` (`self.oldHostageLocation`)))
  (bind _animationidle (`self.animationIdle`))
  (bind _returnvalue (- _oldhostagelocation_z _currenthostagelocation_z))
  (if (or (!= (`KismetMathLibrary.VSize` (`self.GetActorUpVector`)) 0.0) (!= (`KismetMathLibrary.VSize` (`self.GetActorRightVector`)) 0.0))
    (set `self.lastHostageMoveDirection` (select `bool` (> _returnvalue 0.0) :`false` (select `bool` (< _returnvalue 0.0) :`false` (select `bool` (> (- _oldhostagelocation_x _currenthostagelocation_x) 0.0) :`false` "NewEnumerator3" :`true` "NewEnumerator2" :!type "/Game/Blueprints/HostageEnum Enum") :`true` "NewEnumerator1") :`true` "NewEnumerator0")))
  (`PaperFlipbookComponent.SetFlipbook` (`self.Sprite`) (select `bool` (> (`KismetMathLibrary.VSize` (`self.GetVelocity`)) 0.0) :`false` (select `/Game/Blueprints/HostageEnum` (`self.lastHostageMoveDirection`) :`NewEnumerator0` _animationidle :`NewEnumerator1` _animationidle :`NewEnumerator2` _animationidle :`NewEnumerator3` _animationidle) :`true` (select `/Game/Blueprints/HostageEnum` (`self.lastHostageMoveDirection`) :`NewEnumerator0` (`self.animationUp`) :`NewEnumerator1` (`self.animationDown`) :`NewEnumerator2` (`self.animationLeft`) :`NewEnumerator3` (`self.animationRight`)))))

(fn `UserConstructionScript`)