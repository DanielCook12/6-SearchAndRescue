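; Paper2D player character moving on the XZ plane, with HUD widgets, pause menu, health and respawn at its start point.
; Holding left mouse fires FlareProjectiles toward the cursor from limited ammo, with timed reload on R.
; Each tick a fan of line traces becomes canvas triangles drawn to a render target, forming a line-of-sight mask.
; Q spends a flare to temporarily widen sight range and orthographic camera view.
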(event `self.ReceiveBeginPlay`
  (bind _returnvalue (`GameplayStatics.GetPlayerController` 0))
  ;[1 1 1] BeginPlayStuff
  (`|ExecutionSequence`
    (:`then_0`
      ;;[1 1 1] Widget Creation
      (`|ExecutionSequence`
        (:`then_0`
          (bind _returnvalue_2 (`|CreateWidget` "/Game/Blueprints/GUI/AmmoWidget.AmmoWidget_C" _returnvalue)))
        (:`then_1`
          (bind _returnvalue_3 (`|CreateWidget` "/Game/Blueprints/GUI/FlareWidget.FlareWidget_C" _returnvalue)))
        (:`then_2`
          (bind _returnvalue_4 (`|CreateWidget` "/Game/Blueprints/GUI/PlayerHealth.PlayerHealth_C" _returnvalue)))
        (:`then_3`
          (`UserWidget.AddToViewport` _returnvalue_2 0)
          (`UserWidget.AddToViewport` _returnvalue_3 0)
          (`UserWidget.AddToViewport` _returnvalue_4 0))))
    (:`then_1`
      (set `self.Bullets` (`self.MaxBullets`)))
    (:`then_2`
      (set `self.RemainingTime` (`self.TotalTime`)))
    (:`then_3`
      (set `self.Health` (`self.MaxHealth`)))
    (:`then_4`
      (set `self.StartPoint` (`self.K2_GetActorLocation`)))))

(event `Key|Q`
  (params (Key :type "Key Structure"))
  ;[1 1 1] Inputs
  ;;[1 0.4987 0.4787] Flair Thing
  (:`Pressed`
    (if (not (<= (`self.NumOfFlares`) 0))
      (if (`self.CanUseFlair`)
        (set `self.CanUseFlair` false)
        (set `self.NumOfFlares` (- (`self.NumOfFlares`) 1))
        (`/Game/Blueprints/MyModifiedMacros.ForLoopWithDelay` 0 29 0.001
          (:`LoopBody`
            (set `self.LoS-Size` (+ (`self.LoS-Size`) 1.0))
            (`CameraComponent.SetOrthoWidth` (`self.Camera`) (+ (`CameraComponent.OrthoWidth` (`self.Camera`)) 4.0)))
          (:`Completed`
            (`KismetSystemLibrary.Delay` 3.0)
            (`/Game/Blueprints/MyModifiedMacros.ForLoopWithDelay` 0 29 0.05
              (:`LoopBody`
                (set `self.LoS-Size` (- (`self.LoS-Size`) 1.0))
                (`CameraComponent.SetOrthoWidth` (`self.Camera`) (- (`CameraComponent.OrthoWidth` (`self.Camera`)) 4.0)))
              (:`Completed`
                (set `self.CanUseFlair` true)))))
        (else
          (`KismetSystemLibrary.PrintString` "no flair for u")))
      (else
        (`KismetSystemLibrary.PrintString` "Out Of Flairs!!")))))

(event `InputAxis|inputMovementUp`
  (params (AxisValue :type "Float (single-precision)"))
  ;[1 1 1] Inputs
  ;;[1 1 1] Movement
  (if (`self.canMove`)
    (`self.AddMovementInput` (0.0 0.0 1.0) AxisValue)
    (`KismetSystemLibrary.Delay` 0.1)
    (`AudioMixerBlueprintLibrary.PrimeSoundCueForPlayback` "/Game/Sounds/FootSteps/WalkingCue.WalkingCue")
    (`GameplayStatics.SpawnSound2D` "/Game/Sounds/FootSteps/WalkingCue.WalkingCue" 1.0 1.0 0.0 null)))

(event `InputAxis|inputMovementRight`
  (params (AxisValue :type "Float (single-precision)"))
  ;[1 1 1] Inputs
  ;;[1 1 1] Movement
  (if (`self.canMove`)
    (`self.AddMovementInput` (1.0 0.0 0.0) AxisValue)
    (`KismetSystemLibrary.Delay` 0.1)
    (`AudioMixerBlueprintLibrary.PrimeSoundCueForPlayback` "/Game/Sounds/FootSteps/WalkingCue.WalkingCue")
    (`GameplayStatics.SpawnSound2D` "/Game/Sounds/FootSteps/WalkingCue.WalkingCue" 1.0 1.0 0.0 null)))

(event `Key|P`
  (params (Key :type "Key Structure"))
  (bind _returnvalue (`GameplayStatics.GetPlayerController` 0))
  ;[1 1 1] Inputs
  ;;[1 1 1] Pause Menu
  (:`Pressed`
    (`/Engine/EditorBlueprintResources/StandardMacros.FlipFlop` :!label _label
      (:`A`
        (bind _returnvalue_2 (`|CreateWidget` "/Game/Blueprints/GUI/PauseMenu.PauseMenu_C"))
        (`UserWidget.AddToViewport` _returnvalue_2 0)
        (`GameplayStatics.SetGamePaused` true)
        (set `PlayerController.bShowMouseCursor` true _returnvalue))
      (:`B`
        (if (`KismetSystemLibrary.IsValid` _returnvalue_2)
          (`Widget.RemoveFromParent` _returnvalue_2)
          (`GameplayStatics.SetGamePaused` false)
          (set `PlayerController.bShowMouseCursor` false _returnvalue))))))

(event `self.ReceiveTick`
  (params (DeltaSeconds :type "Float (single-precision)"))
  (bind _returnvalue (`self.GetLastMovementInputVector`))
  ;[1 1 1] EventTick
  (`|ExecutionSequence`
    (:`then_0`
      (`self.losVisionSystem`) ; LOS System Function
    )
    (:`then_1`
      (`self.SetFlipbook`) ; Update Animation
    )
    (:`then_2`
      (if (not (== _returnvalue (0.0 0.0 0.0)))
        (set `self.LastMovementInput` (* _returnvalue 90.0))))
    (:`then_3`
      (`PrimitiveComponent.IgnoreActorWhenMoving` (`self.CapsuleComponent`) (`self.SpawnedFlare`) true) ; Ignore Projectile Collision
    )
    (:`then_4`
      (`self.ShootProjectile`))
    (:`then_5`
      (if (`self.TimerActive`)
        (`KismetSystemLibrary.Delay` 0.1)
        (`self.WorkTimer`)))))

(event `Key|V`
  (params (Key :type "Key Structure"))
  ;[1 1 1] Inputs
  (:`Pressed`
    (`self.healthUpdate` 10.0)))

(event `Key|Escape`
  (params (Key :type "Key Structure"))
  ;[1 1 1] Inputs
  ;;[1 1 1] Pause Menu
  (:`Pressed`
    (goto _label)))

(event `healthUpdate`
  (params (`Health Decrease` :type "Float (double-precision)"))
  ;[1 1 1] Inputs
  ;;[1 1 1] Life And Death
  (bind _output_get (set `self.Health` (- (`self.Health`) `Health Decrease`)))
  (if (not (> _output_get 0.0))
    (`self.Perish`)))

(event `Perish`
  ;[1 1 1] Inputs
  ;;[1 1 1] Life And Death
  (set `self.canMove` false)
  (`PaperFlipbookComponent.Stop` (`self.Sprite`))
  (set `self.ShootingEnabled` false)
  (`self.Respawn`))

(event `ShootProjectile`
  (bind _returnvalue (`self.K2_GetActorLocation`))
  (bind (_bblockinghit _binitialoverlap _time _distance _location) (`GameplayStatics.BreakHitResult` (`PlayerController.GetHitResultUnderCursorByChannel` (`GameplayStatics.GetPlayerController` 0) "TraceTypeQuery1" true)))
  ;[1 1 1] Inputs
  ;;[1 1 1] Shooting
  (if (`self.ShootingEnabled`)
    (`/Engine/EditorBlueprintResources/StandardMacros.Gate` true :!label _label_2
      (:`Exit`
        (if (> (`self.Bullets`) 0)
          (`KismetSystemLibrary.Delay` (`self.FireRate`))
          (`|SpawnActorFromClass` "/Game/Blueprints/FlareProjectile.FlareProjectile_C" (`KismetMathLibrary.MakeTransform` _returnvalue (`KismetMathLibrary.FindLookAtRotation` _returnvalue (`KismetMathLibrary.MakeVector` (.x _location) (.y _returnvalue) (.z _location))) (`self.ProjectileScale`)) "Undefined" "OverrideRootScale" null null)
          (`/Engine/EditorBlueprintResources/StandardMacros.DecrementInt` (`self.Bullets`)
            (:`  `
              (`AudioMixerBlueprintLibrary.PrimeSoundCueForPlayback` "/Game/Sounds/GunShots/GunshotCue.GunshotCue")
              (`GameplayStatics.SpawnSound2D` "/Game/Sounds/GunShots/GunshotCue.GunshotCue" 1.0 1.0 0.0 null))))))))

(event `Respawn`
  ;[1 1 1] Inputs
  ;;[1 1 1] Life And Death
  (`KismetSystemLibrary.Delay` 1.0)
  (set `self.Health` (`self.MaxHealth`))
  (`PaperFlipbookComponent.Play` (`self.Sprite`))
  (`self.K2_TeleportTo` (`self.StartPoint`))
  (set `self.canMove` true)
  (set `self.ShootingEnabled` true))

(event `Key|LeftMouseButton`
  (params (Key :type "Key Structure"))
  ;[1 1 1] Inputs
  ;;[1 1 1] Shooting
  (:`Pressed`
    (goto _label_2 :!via `Open`))
  (:`Released`
    (goto _label_2 :!via `Close`)))

(event `BuildTimer`
  (params (TimerName :type String) (TimeIn :type "Float (double-precision)"))
  ;[1 1 1] Inputs
  ;;[1 1 1] Shooting
  ;;;[1 1 1] Reloading
  (set `self.BuildingsTimer` TimerName)
  (set `self.RemainingTime` TimeIn))

(event `Key|R`
  (params (Key :type "Key Structure"))
  (bind _totaltime (`self.TotalTime`))
  ;[1 1 1] Inputs
  ;;[1 1 1] Shooting
  ;;;[1 1 1] Reloading
  (:`Pressed`
    (if (not (== (`self.Bullets`) (`self.MaxBullets`)))
      (set `self.ShootingEnabled` false)
      (set `self.TimerActive` true)
      (`KismetSystemLibrary.Delay` (`self.RemainingTime`))
      (set `self.TimerActive` false)
      (set `self.Bullets` (`self.MaxBullets`))
      (set `self.ShootingEnabled` true)
      (set `self.RemainingTime` _totaltime)
      (if (== _totaltime (- _totaltime 0.1))
        (set `self.RemainingTime` (+ _totaltime 0.1))))))

(event `WorkTimer`
  (bind _remainingtime (`self.RemainingTime`))
  ;[1 1 1] Inputs
  ;;[1 1 1] Shooting
  ;;;[1 1 1] Reloading
  (if (> _remainingtime 0.0)
    (set `self.RemainingTime` (- _remainingtime 0.1))
    (else
      (`self.CountdownComplete`))))

(event `CountdownComplete`
  ;[1 1 1] Inputs
  ;;[1 1 1] Shooting
  ;;;[1 1 1] Reloading
  (set `self.TimerActive` false)
  (`KismetSystemLibrary.K2_ClearTimer` null (`self.BuildingsTimer`)))

(fn `CreateCone`
  (bind _returnvalue (`self.K2_GetActorLocation`))
  (bind _traceresults (`self.TraceResults`))
  (`KismetArrayLibrary.Array_Clear` (`self.TraceResults`))
  (for _index (range (+ (`self.NumTraces`) 1))
    (bind _returnvalue_2 (`KismetMathLibrary.GreaterGreater_VectorRotator` (`KismetMathLibrary.GreaterGreater_VectorRotator` (`self.GetActorForwardVector`) (`KismetMathLibrary.MakeRotator` 0.0 (/ (* (`self.NumTraces`) (`self.DegreesPerTrace`)) -2.0))) (`KismetMathLibrary.MakeRotator` 0.0 (* _index (`self.DegreesPerTrace`)))))
    (bind _returnvalue_3 (+ (* _returnvalue_2 (`self.LoS-Size`)) _returnvalue))
    (bind (_outhit _returnvalue_4) (`KismetSystemLibrary.LineTraceSingle` _returnvalue _returnvalue_3 "TraceTypeQuery1" false (`self.LOS-Ignore`)))
    (if _returnvalue_4
      (bind _returnvalue_5 (* _returnvalue_2 1.0))
      (`KismetArrayLibrary.Array_Add` _traceresults (+ _returnvalue_5 (`.Location` (`GameplayStatics.BreakHitResult` _outhit))))
      (else
        (`KismetArrayLibrary.Array_Add` _traceresults (+ _returnvalue_5 _returnvalue_3))))))

(fn `losVisionSystem`
  (bind _2losrendertarget (`self.2LosRenderTarget`))
  (`|ExecutionSequence`
    (:`then_0`
      (`KismetMaterialLibrary.SetVectorParameterValue` "/Game/Textures/FogOfWar/v3/2PlayerPosition.2PlayerPosition" "PlayerPosition" (`KismetMathLibrary.Conv_VectorToLinearColor` (`self.K2_GetActorLocation`))))
    (:`then_1`
      (`self.CreateCone`))
    (:`then_2`
      (`self.PrepareTrianglesForCanvas`))
    (:`then_3`
      (`KismetRenderingLibrary.ClearRenderTarget2D` _2losrendertarget)
      (bind (_canvas _size _context) (`KismetRenderingLibrary.BeginDrawCanvasToRenderTarget` _2losrendertarget))
      (`Canvas.K2_DrawTriangle` _canvas null (`self.CanvasTriangles`))
      (`KismetRenderingLibrary.EndDrawCanvasToRenderTarget` _context))))

(fn `PrepareTrianglesForCanvas`
  (bind (_returnvalue_x _returnvalue_y _returnvalue_z) (`KismetMathLibrary.BreakVector` (`self.K2_GetActorLocation`)))
  (bind _returnvalue (`KismetMathLibrary.MakeVector` 90.0 90.0))
  (bind _color (`self.Color`))
  (bind _traceresults (`self.TraceResults`))
  (bind _returnvalue_2 (`KismetMathLibrary.MakeVector` _returnvalue_x _returnvalue_z))
  (`KismetArrayLibrary.Array_Clear` (`self.CanvasTriangles`))
  (for _index (range (+ (- (`KismetArrayLibrary.Array_Length` (`self.TraceResults`)) 2) 1))
    (bind (_output_x _output_y _output_z) (`KismetMathLibrary.BreakVector` (`|GetArrayItem` _traceresults _index)))
    (bind (_output_x_2 _output_y_2 _output_z_2) (`KismetMathLibrary.BreakVector` (`|GetArrayItem` _traceresults (+ _index 1))))
    (`KismetArrayLibrary.Array_Add` (`self.CanvasTriangles`) (make `CanvasUVTri` (`KismetMathLibrary.Conv_VectorToVector2D` _returnvalue) (0.0 0.0) _color (`KismetMathLibrary.Conv_VectorToVector2D` (+ (- (`KismetMathLibrary.MakeVector` _output_x _output_z) _returnvalue_2) _returnvalue)) (0.0 0.0) _color (`KismetMathLibrary.Conv_VectorToVector2D` (+ (- (`KismetMathLibrary.MakeVector` _output_x_2 _output_z_2) _returnvalue_2) _returnvalue)) (0.0 0.0) _color))))

(fn `SetFlipbook`
  (bind _animationidle (`self.AnimationIdle`))
  (if (or (!= (`self.GetInputAxisValue`) 0.0) (!= (`self.GetInputAxisValue`) 0.0))
    (set `self.LastMoveDirection` (select `bool` (> (`self.GetInputAxisValue`) 0.0) :`false` (select `bool` (< (`self.GetInputAxisValue`) 0.0) :`false` (select `bool` (> (`self.GetInputAxisValue`) 0.0) :`false` "NewEnumerator2" :`true` "NewEnumerator3" :!type "/Game/Blueprints/MoveEnum Enum") :`true` "NewEnumerator1") :`true` "NewEnumerator0")))
  (`PaperFlipbookComponent.SetFlipbook` (`self.Sprite`) (select `bool` (> (`KismetMathLibrary.VSize` (`self.GetVelocity`)) 0.0) :`false` (select `/Game/Blueprints/MoveEnum` (`self.LastMoveDirection`) :`NewEnumerator0` _animationidle :`NewEnumerator1` _animationidle :`NewEnumerator2` _animationidle :`NewEnumerator3` _animationidle) :`true` (select `/Game/Blueprints/MoveEnum` (`self.LastMoveDirection`) :`NewEnumerator0` (`self.AnimationUp`) :`NewEnumerator1` (`self.AnimationDown`) :`NewEnumerator2` (`self.AnimationLeft`) :`NewEnumerator3` (`self.AnimationRight`)))))

(fn `UserConstructionScript`)