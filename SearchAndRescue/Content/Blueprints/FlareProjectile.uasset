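; Flare projectile that flies briefly, then halts in place, and destroys itself shortly after hitting anything other than the player.
; On spawn it joins the player character's LOSIgnore list, sets its sprite and collision to ignore the player, and starts a timed stop.
; The timer and hit event set a StopMove flag, which makes Tick halt ProjectileMovement every frame.
; Overlaps only print the other actor's name.
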(event `self.ReceiveBeginPlay`
  (`|ExecutionSequence`
    (:`then_0`
      (bind _asplayer_character (cast `/Game/Blueprints/PlayerCharacter` (`GameplayStatics.GetPlayerCharacter` 0)))
      (`KismetArrayLibrary.Array_Add` (`/Game/Blueprints/PlayerCharacter.LOS-Ignore` _asplayer_character) self))
    (:`then_1`
      (`PrimitiveComponent.IgnoreActorWhenMoving` (`self.PaperSprite`) (`GameplayStatics.GetPlayerCharacter` 0) true)
      (`PrimitiveComponent.IgnoreActorWhenMoving` (`self.MainCollision`) (`GameplayStatics.GetPlayerCharacter` 0) true))
    (:`then_2`
      (`KismetSystemLibrary.Delay` 1.0)
      (set `self.StopMove` true))))

(event `self.ReceiveTick`
  (params (DeltaSeconds :type "Float (single-precision)"))
  (if (`self.StopMove`)
    (`MovementComponent.StopMovementImmediately` (`self.ProjectileMovement`))))

(event `self.MainCollision.OnComponentHit`
  (params (HitComponent :type "PrimitiveComponent Object Reference") (OtherActor :type "Actor Object Reference") (OtherComp :type "PrimitiveComponent Object Reference") (NormalImpulse :type "Vector Structure") (Hit :type "HitResult Structure (by ref)"))
  (if (not (== OtherActor (`GameplayStatics.GetPlayerCharacter` 0)))
    (set `self.StopMove` true)
    (`KismetSystemLibrary.Delay` 0.2)
    (`self.K2_DestroyActor`)))

(event `self.MainCollision.OnComponentBeginOverlap`
  (params (OverlappedComponent :type "PrimitiveComponent Object Reference") (OtherActor :type "Actor Object Reference") (OtherComp :type "PrimitiveComponent Object Reference") (OtherBodyIndex :type Integer) (bFromSweep :type Boolean) (SweepResult :type "HitResult Structure (by ref)"))
  (`KismetSystemLibrary.PrintString` (`KismetSystemLibrary.GetDisplayName` OtherActor)))

(fn `UserConstructionScript`)