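; BreadTeleporter is an actor that teleports the player character to a matching TelePoint and advances the player's level.
; On player overlap with its collision component, it searches all TelePoint actors for one whose TelepointID equals its TeleporterID.
; It teleports the player there with zeroed rotation, then steps CurrentLevel from Level1 to Level2 or Level2 to Level3, saving that location as StartPoint.
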(event `self.CollisionComponent.OnComponentBeginOverlap`
  (params (OverlappedComponent :type "PrimitiveComponent Object Reference") (OtherActor :type "Actor Object Reference") (OtherComp :type "PrimitiveComponent Object Reference") (OtherBodyIndex :type Integer) (bFromSweep :type Boolean) (SweepResult :type "HitResult Structure (by ref)"))
  (if (== OtherActor (`GameplayStatics.GetPlayerCharacter` 0))
    (cast `/Game/Blueprints/PlayerCharacter` (`GameplayStatics.GetPlayerCharacter` 0))
    (bind _outactors (`GameplayStatics.GetAllActorsOfClass` "/Game/Blueprints/TelePoint.TelePoint_C"))
    (for _array_element _outactors
      (if (== (`/Game/Blueprints/TelePoint.telepointID` _array_element) (`self.teleporterID`))
        (set `self.TeleOutput` _array_element)))
    (`/Engine/EditorBlueprintResources/StandardMacros.IsValid` (`self.TeleOutput`)
      (:`Is Valid`
        (bind _astele_point (cast `/Game/Blueprints/TelePoint` (`self.TeleOutput`)))
        (bind _asplayer_character (cast `/Game/Blueprints/PlayerCharacter` (`GameplayStatics.GetPlayerCharacter` 0)))
        (bind _returnvalue (`self.K2_GetActorLocation` _astele_point))
        (`self.K2_TeleportTo` :`self` _asplayer_character :`DestLocation` _returnvalue)
        (bind _currentlevel (`/Game/Blueprints/PlayerCharacter.CurrentLevel` _asplayer_character))
        (if (== _currentlevel "Level1")
          (set `/Game/Blueprints/PlayerCharacter.CurrentLevel` "Level2" _asplayer_character)
          (set `/Game/Blueprints/PlayerCharacter.StartPoint` _returnvalue _asplayer_character :!label _label)
          (elif (== _currentlevel "Level2")
            (set `/Game/Blueprints/PlayerCharacter.CurrentLevel` "Level3" _asplayer_character)
            (goto _label)))))))

(fn `UserConstructionScript`
  (`parent.UserConstructionScript`))