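; HostageCollector2 is a drop-off actor that ends the game when the player arrives holding all three hostages.
; Begin and end overlap events track whether the player character is inside.
; While inside, Tick polls the PlayerCharacter's three holding flags and calls its EndGame when all are true.
; Otherwise three text renders show which hostages are missing, and they are not cleared when the player leaves.
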(event `self.ReceiveActorBeginOverlap`
  (params (OtherActor :type "Actor Object Reference"))
  (if (== OtherActor (`GameplayStatics.GetPlayerCharacter` 0))
    (set `self.PlayerOverlapping` true)))

(event `self.ReceiveActorEndOverlap`
  (params (OtherActor :type "Actor Object Reference"))
  (if (== OtherActor (`GameplayStatics.GetPlayerCharacter` 0))
    (set `self.PlayerOverlapping` false)))

(event `self.ReceiveTick`
  (params (DeltaSeconds :type "Float (single-precision)"))
  (bind _textrender1 (`self.TextRender1`))
  (bind _textrender2 (`self.TextRender2`))
  (bind _textrender3 (`self.TextRender3`))
  (if (`self.PlayerOverlapping`)
    (bind _asplayer_character (cast `/Game/Blueprints/PlayerCharacter` (`GameplayStatics.GetPlayerCharacter` 0)))
    (bind _isholdinghostage1 (`/Game/Blueprints/PlayerCharacter.IsHoldingHostage1` _asplayer_character))
    (bind _isholdinghostage2 (`/Game/Blueprints/PlayerCharacter.IsHoldingHostage2` _asplayer_character))
    (bind _isholdinghostage3 (`/Game/Blueprints/PlayerCharacter.IsHoldingHostage3` _asplayer_character))
    (if (and (and _isholdinghostage1 _isholdinghostage2) _isholdinghostage3)
      (`/Game/Blueprints/PlayerCharacter.EndGame` _asplayer_character)
      (else
        (if _isholdinghostage1
          (`TextRenderComponent.K2_SetText` _textrender1 (`KismetTextLibrary.Conv_StringToText` ""))
          (else
            (`TextRenderComponent.K2_SetText` _textrender1 (`KismetTextLibrary.Conv_StringToText` "Missing Hostage #1"))))
        (if _isholdinghostage2
          (`TextRenderComponent.K2_SetText` _textrender2 (`KismetTextLibrary.Conv_StringToText` ""))
          (else
            (`TextRenderComponent.K2_SetText` _textrender2 (`KismetTextLibrary.Conv_StringToText` "Missing Hostage #2"))))
        (if _isholdinghostage3
          (`TextRenderComponent.K2_SetText` _textrender3 (`KismetTextLibrary.Conv_StringToText` ""))
          (else
            (`TextRenderComponent.K2_SetText` _textrender3 (`KismetTextLibrary.Conv_StringToText` "Missing Hostage #3"))))))))

(fn `UserConstructionScript`)