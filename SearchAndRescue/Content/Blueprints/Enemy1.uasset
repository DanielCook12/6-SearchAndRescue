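; Enemy AI for a Paper2D character that patrols, chases and shoots the player in the XZ plane.
; InterpToMovement patrols three construction-script points until DetectShphere overlap deactivates it and movement input drives the chase.
; AttackSphere overlap halts the chase and loops delayed EnemyProjectile spawns aimed at the player.
; Tick picks directional flipbooks from frame-to-frame location change, and EnemyHealthUpdate decrements health or destroys the actor at zero.
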(event `self.ReceiveTick`
  (params (DeltaSeconds :type "Float (single-precision)"))
  (bind _returnvalue (`self.K2_GetActorLocation`))
  (bind (_returnvalue_x _returnvalue_y _returnvalue_z) (`KismetMathLibrary.BreakVector` (`SceneComponent.K2_GetComponentLocation` (`self.CapsuleComponent`))))
  ;[1 1 1] Enemy AI
  (`/Engine/EditorBlueprintResources/StandardMacros.IsValid` self
    (:`Is Valid`
      (`|ExecutionSequence`
        (:`then_0`
          (`|ExecutionSequence`
            (:`then_0`
              (`self.PlayerCharacterLocationUpdate`))
            (:`then_1`
              (set `self.oldActorLocation` _returnvalue))
            (:`then_2`
              (`KismetSystemLibrary.Delay` DeltaSeconds)
              (set `self.currentActorLocation` _returnvalue))))
        (:`then_1`
          (`self.enemyAnimUpdate`))
        (:`then_2`
          (if (`self.isOverlapping`)
            (`ActorComponent.Deactivate` (`self.InterpToMovement`))))
        (:`then_3`
          (if (`self.isOverlappingAttack`)
            (`self.AddMovementInput` (0.0 0.0 0.0) 0.0)
            (elif (`self.isOverlapping`)
              (bind _asplayer_character (cast `/Game/Blueprints/PlayerCharacter` (`GameplayStatics.GetPlayerCharacter` 0)))
              (bind (_returnvalue_x_2 _returnvalue_y_2 _returnvalue_z_2) (`KismetMathLibrary.BreakVector` (`SceneComponent.K2_GetComponentLocation` (`Character.CapsuleComponent` _asplayer_character))))
              (`self.AddMovementInput` (`KismetMathLibrary.MakeVector` (- _returnvalue_x_2 _returnvalue_x) 0.0 (- _returnvalue_z_2 _returnvalue_z)))
              (else
                (`self.AddMovementInput` (0.0 0.0 0.0) 0.0)))))))))

(event `self.InterpToMovement.OnInterpToReverse`
  (params (ImpactResult :type "HitResult Structure (by ref)") (Time :type "Float (single-precision)"))
  (bind _sprite (`self.Sprite`))
  (`/Engine/EditorBlueprintResources/StandardMacros.FlipFlop`
    (:`A`
      (`SceneComponent.K2_SetWorldRotation` :`self` _sprite))
    (:`B`
      (`SceneComponent.K2_SetWorldRotation` _sprite (struct :`Yaw` 180.0) false false))))

(event `Enemy Health Update`
  (if (> (`self.enemyHealth`) 0)
    (bind _result (`/Engine/EditorBlueprintResources/StandardMacros.DecrementInt` (`self.enemyHealth`))
      (:`  `
        (`KismetSystemLibrary.PrintString` (`KismetStringLibrary.Conv_IntToString` _result))))
    (else
      (`KismetSystemLibrary.PrintString` "ded")
      (`ActorComponent.K2_DestroyComponent` (`self.Sprite`))
      (if true
        (`self.K2_DestroyActor`)))))

(event `self.detectShphere.OnComponentBeginOverlap`
  (params (OverlappedComponent :type "PrimitiveComponent Object Reference") (OtherActor :type "Actor Object Reference") (OtherComp :type "PrimitiveComponent Object Reference") (OtherBodyIndex :type Integer) (bFromSweep :type Boolean) (SweepResult :type "HitResult Structure (by ref)"))
  ;[1 1 1] Player Character Detection
  (bind _output_get (set `self.PlayerCharacter` OtherActor))
  (cast `/Game/Blueprints/PlayerCharacter` _output_get)
  (set `self.isOverlapping` true))

(event `EnemyProjectileSpawn`
  (bind (_returnvalue_x _returnvalue_y _returnvalue_z) (`KismetMathLibrary.BreakVector` (`self.K2_GetActorLocation`)))
  (bind (_returnvalue_x_2 _returnvalue_y_2 _returnvalue_z_2) (`KismetMathLibrary.BreakVector` (`self.K2_GetActorLocation` (`GameplayStatics.GetPlayerCharacter` 0))))
  (bind _returnvalue (`|SpawnActorFromClass` "/Game/Blueprints/EnemyProjectile.EnemyProjectile_C" (`KismetMathLibrary.MakeTransform` (`KismetMathLibrary.MakeVector` _returnvalue_x (+ _returnvalue_y 12.0) _returnvalue_z) (`KismetMathLibrary.FindLookAtRotation` (`KismetMathLibrary.MakeVector` _returnvalue_x _returnvalue_y _returnvalue_z) (`KismetMathLibrary.MakeVector` _returnvalue_x_2 0.0 _returnvalue_z_2)) (1.0 1.0 1.0)) "Undefined" "OverrideRootScale" null null))
  (bind _asenemy_projectile (cast `/Game/Blueprints/EnemyProjectile` _returnvalue))
  (`/Game/Blueprints/EnemyProjectile.getEnemy` _asenemy_projectile self))

(event `self.detectShphere.OnComponentEndOverlap`
  (params (OverlappedComponent :type "PrimitiveComponent Object Reference") (OtherActor :type "Actor Object Reference") (OtherComp :type "PrimitiveComponent Object Reference") (OtherBodyIndex :type Integer))
  ;[1 1 1] Player Character Detection
  (cast `/Game/Blueprints/PlayerCharacter` OtherActor)
  (set `self.isOverlapping` false))

(event `self.attackSphere.OnComponentBeginOverlap`
  (params (OverlappedComponent :type "PrimitiveComponent Object Reference") (OtherActor :type "Actor Object Reference") (OtherComp :type "PrimitiveComponent Object Reference") (OtherBodyIndex :type Integer) (bFromSweep :type Boolean) (SweepResult :type "HitResult Structure (by ref)"))
  ;[1 1 1] Player Character Detection
  (cast `/Game/Blueprints/PlayerCharacter` OtherActor)
  (bind _output_get (set `self.isOverlappingAttack` true))
  (if _output_get :!label _label
    (`KismetSystemLibrary.Delay` 1.0)
    (`self.EnemyProjectileSpawn`)
    (goto _label)))

(event `self.attackSphere.OnComponentEndOverlap`
  (params (OverlappedComponent :type "PrimitiveComponent Object Reference") (OtherActor :type "Actor Object Reference") (OtherComp :type "PrimitiveComponent Object Reference") (OtherBodyIndex :type Integer))
  ;[1 1 1] Player Character Detection
  (cast `/Game/Blueprints/PlayerCharacter` OtherActor)
  (set `self.isOverlappingAttack` false))

(event `PlayerCharacterLocationUpdate`
  (bind _playercharacter (`self.PlayerCharacter`))
  (`/Engine/EditorBlueprintResources/StandardMacros.IsValid` _playercharacter
    (:`Is Valid`
      (set `self.PlayerCharacterLocation` (`self.K2_GetActorLocation` _playercharacter)))))

(fn `enemyAnimUpdate`
  (bind (_currentactorlocation_x _currentactorlocation_y _currentactorlocation_z) (`KismetMathLibrary.BreakVector` (`self.currentActorLocation`)))
  (bind (_oldactorlocation_x _oldactorlocation_y _oldactorlocation_z) (`KismetMathLibrary.BreakVector` (`self.oldActorLocation`)))
  (bind _animationidle (`self.animationIdle`))
  (bind _returnvalue (- _oldactorlocation_z _currentactorlocation_z))
  (if (or (!= (`KismetMathLibrary.VSize` (`self.GetActorUpVector`)) 0.0) (!= (`KismetMathLibrary.VSize` (`self.GetActorRightVector`)) 0.0))
    (set `self.lastEnemyMoveDirection` (select `bool` (> _returnvalue 0.0) :`false` (select `bool` (< _returnvalue 0.0) :`false` (select `bool` (> (- _oldactorlocation_x _currentactorlocation_x) 0.0) :`false` "NewEnumerator3" :`true` "NewEnumerator2" :!type "/Game/Blueprints/Enemy1Enum Enum") :`true` "NewEnumerator1") :`true` "NewEnumerator0")))
  (`PaperFlipbookComponent.SetFlipbook` (`self.Sprite`) (select `bool` (> (`KismetMathLibrary.VSize` (`self.GetVelocity`)) 0.0) :`false` (select `/Game/Blueprints/Enemy1Enum` (`self.lastEnemyMoveDirection`) :`NewEnumerator0` _animationidle :`NewEnumerator1` _animationidle :`NewEnumerator2` _animationidle :`NewEnumerator3` _animationidle) :`true` (select `/Game/Blueprints/Enemy1Enum` (`self.lastEnemyMoveDirection`) :`NewEnumerator0` (`self.animationUp`) :`NewEnumerator1` (`self.animationDown`) :`NewEnumerator2` (`self.animationLeft`) :`NewEnumerator3` (`self.animationRight`)))))

(fn `UserConstructionScript`
  (set `InterpToMovementComponent.ControlPoints` (`|MakeArray` (make `InterpControlPoint` (`self.Point A`)) (make `InterpControlPoint` (`self.Point B`)) (make `InterpControlPoint` (`self.Point C`))) (`self.InterpToMovement`)))